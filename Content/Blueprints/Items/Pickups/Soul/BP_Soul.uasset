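; BP_Soul is a soul pickup item whose own graphs currently run no logic, as BeginPlay, Tick and the construction script are empty.
; Disconnected nodes, marked as old code, once traced downward against WorldStatic to set a hover height above the ground and slowly lowered the actor to it.
; Any active pickup behavior is not defined in these graphs.
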(event EventBeginPlay
  ;[1 1 1] Just Old Code
)

(event EventTick
  (params (DeltaSeconds :type Float%20%28single-precision%29))
  ;[1 1 1] Just Old Code
)

(fn ConstructionScript)