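; BP_RaptorWeapon is a weapon Blueprint that applies Chaos physics fields to break and scatter destructible objects at a given location.
; Its CreateFields event applies a radial falloff external cluster strain to fracture geometry collections, waits briefly, then applies a radial vector linear force to push the pieces outward.
; BeginPlay, Tick and the construction script are empty, and a debug sphere draw is left unconnected.
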(event EventBeginPlay)

(event EventCreateFields
  (params (FieldLocation :type Vector%20%28by%20ref%29 :default "0, 0, 0"))
  (Class|FieldSystemComponent|ApplyPhysicsField (Variables|Default|GetFieldSystem) true "Field_ExternalClusterStrain" 0 (Field|SetRadialFalloff (Variables|Default|GetRadialFalloff) 1e+06 0.8 1.0 0.0 1.2e+02 FieldLocation "Field_FallOff_None"))
  (Utilities|FlowControl|Delay 0.01)
  (Class|FieldSystemComponent|ApplyPhysicsField (Variables|Default|GetFieldSystem) true "Field_LinearForce" (Variables|Default|GetFieldSystemMetaDataFilter) (Field|SetRadialVector (Variables|Default|GetRadialVector) 3.5e+05 FieldLocation)))

(event EventTick
  (params (DeltaSeconds :type Float%20%28single-precision%29)))

(fn ConstructionScript)